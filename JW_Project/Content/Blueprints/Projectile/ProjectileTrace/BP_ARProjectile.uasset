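; Assault rifle projectile Blueprint that is switched on and off through activate and deactivate events rather than spawned or destroyed here.
; On activation it shows the bullet, launches it along local forward at its projectile speed, enables query-only collision and starts a lifetime timer.
; Deactivation hides the bullet, stops movement, disables collision and clears the timer.
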(event EventOnActivate
  (bind _projectilemovement (Variables|Default|GetProjectileMovement))
  (Rendering|SetVisibility (Variables|Default|GetBulletProjectile) true false)
  (Game|Components|ProjectileMovement|SetVelocityinLocalSpace _projectilemovement (* (Class|KismetMathLibrary|VectorForward) (Variables|Default|GetProjectile%20Speed)))
  (Components|Activation|Activate _projectilemovement false)
  (Collision|SetCollisionEnabled (Variables|Default|GetBulletProjectile) "QueryOnly")
  (bind _returnvalue (Utilities|Time|SetTimerbyEvent (EventDispatchers|CreateEvent :!event OnDeactivate) (Variables|Default|GetLifeTime)))
  (Variables|Default|SetTimer _returnvalue))

(event EventOnDeactivate
  (Rendering|SetVisibility (Variables|Default|GetBulletProjectile) false false)
  (Components|Activation|Deactivate (Variables|Default|GetProjectileMovement))
  (Collision|SetCollisionEnabled (Variables|Default|GetBulletProjectile) "NoCollision")
  (Utilities|Time|ClearandInvalidateTimerbyHandle (Variables|Default|GetTimer)))

(fn ConstructionScript
  (|CallParentFunction))