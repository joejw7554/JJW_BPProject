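; BP_SpawnManager runs wave-based enemy spawning and fires OnGameVictory once the final wave is cleared.
; On BeginPlay it gathers all BP_SpawnArea actors, then a looping timer spawns random enemy classes at random areas with BT_EnemyBase until the wave's count is spent.
; Each enemy's death dispatcher decrements the remaining count.
; At zero, the next wave starts after a short delay with three more enemies than the last.
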(event Custom|ActivateSpawn
  (bind _returnvalue (Utilities|Time|SetTimerbyEvent (delegate Custom|StartSpawn) (Variables|Default|GetSpawnInterval) true false 1.0))
  (Variables|Default|SetTimerHandle _returnvalue))

(event Custom|CheckNextWave
  (if (== (Variables|Default|GetCurrentWaveLevel) (Variables|Default|GetMaxWaveLevel))
    (Utilities|Time|ClearandInvalidateTimerbyHandle (Variables|Default|GetTimerHandle))
    (CallFunction|TheEnd)
    (else
      (Math|Integer|IncrementInt (Variables|Default|GetCurrentWaveLevel)
        (:%20%20
          (Utilities|Time|ClearandInvalidateTimerbyHandle (Variables|Default|GetTimerHandle))
          (bind _output_get (Variables|Default|SetSpawnCount (+ (Variables|Default|GetPreviousSpawnCount) 3)))
          (bind _output_get_2 (Variables|Default|SetRemainingEnemies _output_get))
          (Variables|Default|SetPreviousSpawnCount _output_get_2)
          (Utilities|FlowControl|Delay 3.0)
          (CallFunction|ActivateSpawn))))))

(event Custom|StartSpawn
  (if (!= (Variables|Default|GetSpawnCount) 0)
    (CallFunction|SpawnEnemy)
    (else
      (CallFunction|StopSpawn))))

(event Custom|StopSpawn
  (Utilities|Time|ClearandInvalidateTimerbyHandle (Variables|Default|GetTimerHandle)))

(event Custom|InitialSetup
  (bind _outactors (Actor|GetAllActorsOfClass "/Game/Blueprints/Spawn/BP_SpawnArea.BP_SpawnArea_C"))
  (for _array_element _outactors
    (Utilities|Array|Add (Variables|Default|GetSpawnAreaList) _array_element))
  (Variables|Default|SetSpawnAreaMaxIndex (- (Utilities|Array|Length (Variables|Default|GetSpawnAreaList)) 1))
  (Variables|Default|SetEnemyTypeMaxIndex (- (Utilities|Array|Length (Variables|Default|GetEnemyClass)) 1)))

(event Custom|SpawnEnemy
  (bind _returnvalue (AI|SpawnAIFromClass (Utilities|Array|Get(acopy) (Variables|Default|GetEnemyClass) (Math|Random|RandomIntegerinRange 0 (Variables|Default|GetEnemyTypeMaxIndex))) "/Game/Blueprints/Enemy/AI/BT_EnemyBase.BT_EnemyBase" (Transformation|GetActorLocation (Utilities|Array|Get(acopy) (Variables|Default|GetSpawnAreaList) (Math|Random|RandomIntegerinRange 0 (Variables|Default|GetSpawnAreaMaxIndex)))) "0, 0, 0" false self))
  (bind _asbp_base_enemy (Utilities|Casting|CastToBP_BaseEnemy _returnvalue))
  (EventDispatchers|BindEventtoOnEnemyDeadCount _asbp_base_enemy (delegate Custom|DecreaseRemaingCount))
  (Math|Integer|DecrementInt (Variables|Default|GetSpawnCount)))

(event Custom|DecreaseRemaingCount
  (bind _result (Math|Integer|DecrementInt (Variables|Default|GetRemainingEnemies))
    (:%20%20
      (if (== _result 0)
        (CallFunction|CheckNextWave)))))

(event Custom|TheEnd
  ;[0.15 0.15 0.15 0.5] UI Should Come here
  (Utilities|Time|ClearandInvalidateTimerbyHandle (Variables|Default|GetTimerHandle))
  (Default|CallOnGameVictory))

(event EventBeginPlay
  (Utilities|FlowControl|Sequence
    (:then_0
      (CallFunction|InitialSetup)
      (bind _output_get (Variables|Default|SetRemainingEnemies (Variables|Default|GetSpawnCount)))
      (Variables|Default|SetPreviousSpawnCount _output_get))
    (:then_1
      (CallFunction|ActivateSpawn))))

(fn ConstructionScript)