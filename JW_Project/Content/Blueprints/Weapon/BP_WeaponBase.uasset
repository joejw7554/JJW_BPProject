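; Base weapon Blueprint that fires hitscan shots and damages actors tagged Enemy.
; On BeginPlay it gets an arrow component from the player pawn through a message call, using it as the aim origin and direction.
; Fire runs a debug-drawn Visibility line trace over the weapon range, attaches a muzzle flash at the gun's socket and spawns a projectile-trace actor at the arrow.
; The sound event is an empty stub.
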(event Custom|Fire
  (CallFunction|LineTrace)
  (CallFunction|PlayVFX)
  (CallFunction|PlaySFX)
  (CallFunction|SpawnProjectileTrace))

(event Custom|LineTrace
  (bind _raycaststartdirection (Variables|Default|GetRayCastStartDirection))
  (bind _returnvalue (Transformation|GetWorldLocation _raycaststartdirection))
  (bind _outhit (Collision|LineTraceByChannel _returnvalue (+ _returnvalue (* (Math|Vector|GetForwardVector (Transformation|GetWorldRotation _raycaststartdirection)) (Variables|Default|GetWeaponRange))) "TraceTypeQuery1" false 0 "ForDuration"))
  (Utilities|IsValid (.hitactor _outhit)
    (:Is%20Valid
      (if (Actor|ActorHasTag (.hitactor _outhit) "Enemy")
        (Game|Damage|ApplyDamage (.hitactor _outhit) (Variables|Default|GetWeaponDamage) 0 self "/Script/Engine.DamageType")))))

(event Custom|PlayVFX
  (Effects|SpawnEmitterAttached "/Game/MilitaryWeapSilver/FX/P_AssaultRifle_MuzzleFlash.P_AssaultRifle_MuzzleFlash" (Variables|Default|GetGunMesh) "MuzzleSocket" "0, 0, 0" "0, 0, 0" "1.000000,1.000000,1.000000" "SnapToTarget"))

(event Custom|PlaySFX)

(event Custom|SpawnProjectileTrace
  (Game|SpawnActorfromClass "/Game/Blueprints/Actors/ProjectileTrace/BP_ProjectileTrace.BP_ProjectileTrace_C" (Transformation|GetWorldTransform (Variables|Default|GetRayCastStartDirection)) "AlwaysSpawn" "MultiplyWithRoot" 0 0))

(event EventBeginPlay
  (bind _arrowcomp (Class|BPIPlayer|GetArrowComponent(Message) (Game|Player|GetPlayerPawn 0)))
  (Variables|Default|SetRayCastStartDirection _arrowcomp))

(fn ConstructionScript)