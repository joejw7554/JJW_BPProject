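; Actor component that pools reusable actors of a configurable class, likely trace projectiles, for its owning actor.
; On BeginPlay it prespawns a set quantity, deactivates each, attaches it to the owner at a reset location and binds its return-to-pool event.
; GetObject takes the first pooled actor, moves it to the requested transform and activates it.
; An empty pool grows by spawning another actor and retrying recursively.
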(event Custom|SpawnObjectToPool
  (bind _returnvalue (Game|SpawnActorfromClass (Variables|Default|GetClassToSpawn) (Math|Transform|MakeTransform "0, 0, 0" "0, 0, 0" "1.000000,1.000000,1.000000") "Undefined" "MultiplyWithRoot" (Components|GetOwner) 0))
  (Class|BPIPoolOptions|Deactivate(Message) _returnvalue)
  (CallFunction|MoveChildtoPool _returnvalue)
  (EventDispatchers|BindEventtoOnObjectReturntoPool _returnvalue (delegate Custom|MoveChildToPool)))

(event Custom|MoveChildToPool
  (params (ToPool :type BP%20Base%20Projectile%20Object%20Reference))
  (Transformation|AttachActorToActor ToPool (Components|GetOwner) "None" "SnapToTarget" "SnapToTarget" "SnapToTarget" true)
  (Transformation|SetActorRelativeLocation ToPool (Variables|Default|GetResetLocation))
  (Utilities|Array|Add (Variables|Default|GetProjectilePool) ToPool))

(event EventBeginPlay
  (Utilities|Array|Clear (Variables|Default|GetProjectilePool))
  (for _index (range 0 (- (Variables|Default|GetProjectileQuanity) 1))
    (CallFunction|SpawnObjecttoPool)))

(fn GetObject
  (params (SpawnTransform :type Transform%20%28by%20ref%29))
  (if (> (Utilities|Array|Length (Variables|Default|GetProjectilePool)) 0)
    (bind _output_get (LocalVariables|SetResult (Utilities|Array|Get(acopy) (Variables|Default|GetProjectilePool))))
    (Utilities|Array|RemoveItem (Variables|Default|GetProjectilePool) _output_get)
    (Transformation|SetActorTransform _output_get SpawnTransform)
    (Default|Activate (LocalVariables|GetResult))
    (return (LocalVariables|GetResult))
    (else
      (CallFunction|SpawnObjecttoPool)
      (bind _newobject (CallFunction|GetObject SpawnTransform))
      (return _newobject))))