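; Pooled projectile actor that toggles between active and inactive states for reuse.
; On activation it shows the bullet component, launches the projectile movement along local forward at the configured speed and starts a lifetime timer.
; On deactivation it hides the bullet and stops the movement component.
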(event EventOnActivate
  (bind _projectilemovement (Variables|Default|GetProjectileMovement))
  (Rendering|SetVisibility (Variables|Default|GetBulletProjectile) true false)
  (Game|Components|ProjectileMovement|SetVelocityinLocalSpace _projectilemovement (* (Class|KismetMathLibrary|VectorForward) (Variables|Default|GetProjectile%20Speed)))
  (Components|Activation|Activate _projectilemovement false)
  (Utilities|Time|SetTimerbyEvent (EventDispatchers|CreateEvent :!event OnDeactivate) (Variables|Default|GetLifeTime)))

(event EventOnDeactivate
  (Rendering|SetVisibility (Variables|Default|GetBulletProjectile) false false)
  (Components|Activation|Deactivate (Variables|Default|GetProjectileMovement)))

(fn ConstructionScript
  (|CallParentFunction))