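; Actor component that pools BP_ProjectileTrace actors for reuse.
; On BeginPlay it spawns a row of deactivated projectiles and, if its owner is a BP_ProjectileTrace, binds RemoveOrAdd to that owner's pool event.
; PullProjectile removes and activates the first pooled projectile, or takes a spawn-on-demand path when the pool is empty.
; RemoveOrAdd also handles returns, re-adding and deactivating the projectile at a given location.
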(event Custom|CreateProjectilePool
  (for _index (range 0 (- (Variables|Default|GetProjectileQuanity) 1))
    (bind _returnvalue (Game|SpawnActorfromClass "/Game/Blueprints/Actors/ProjectileTrace/BP_ProjectileTrace.BP_ProjectileTrace_C" (Math|Transform|MakeTransform (Math|Vector|MakeVector 5e+03 (Math|Conversions|ToFloat(Integer) (* _index 150)) 8e+02) "0, 0, 0" "1.000000,1.000000,1.000000") "AlwaysSpawn" "MultiplyWithRoot" 0 0))
    (Default|DeactivateProjectile _returnvalue (Variables|Default|GetResetLocation))
    (Utilities|Array|Add (Variables|Default|GetProjectilePool) _returnvalue)))

(event Custom|RemoveOrAdd
  (params (ProjectileToPass :type BP%20Projectile%20Trace%20Object%20Reference) (WantToAddBack :type Boolean) (ProjectileActivateLocation :type Vector))
  (if WantToAddBack
    (Utilities|Array|Add (Variables|Default|GetProjectilePool) ProjectileToPass)
    (Default|DeactivateProjectile ProjectileToPass ProjectileActivateLocation)
    (else
      ;[0.15 0.15 0.15 0.5] 현재 벡터에 남아있는거 쓴다
      (CallFunction|RemoveandActivate))))

(event Custom|PullProjectile
  (params (ActivateLocation :type Vector%20%28by%20ref%29))
  (bind _projectilepool (Variables|Default|GetProjectilePool))
  (if (> (Utilities|Array|Length _projectilepool) 0)
    (CallFunction|RemoveorAdd (Utilities|Array|Get(acopy) _projectilepool) false ActivateLocation)
    (else
      (CallFunction|CreateNewandActivate))))

(event Custom|CreateNewAndActivate
  (bind _projectilepool (Variables|Default|GetProjectilePool))
  (bind _returnvalue (Game|SpawnActorfromClass "/Game/Blueprints/Actors/ProjectileTrace/BP_ProjectileTrace.BP_ProjectileTrace_C" (Math|Transform|MakeTransform "0.000000,0.000000,800.000000" "0, 0, 0" "1.000000,1.000000,1.000000") "AlwaysSpawn" "MultiplyWithRoot" 0 0))
  (bind _returnvalue_2 (Utilities|Array|Add _projectilepool _returnvalue))
  (Utilities|Array|RemoveItem _projectilepool (Utilities|Array|Get(acopy) _projectilepool _returnvalue_2))
  (Default|ActivateProjectile (stale Custom|RemoveOrAdd ProjectileToPass) (stale Custom|RemoveOrAdd ProjectileActivateLocation)))

(event Custom|RemoveAndActivate
  (Utilities|Array|RemoveItem (Variables|Default|GetProjectilePool) (stale Custom|RemoveOrAdd ProjectileToPass))
  (Default|ActivateProjectile (stale Custom|RemoveOrAdd ProjectileToPass) (stale Custom|RemoveOrAdd ProjectileActivateLocation)))

(event EventBeginPlay
  (Utilities|FlowControl|Sequence
    (:then_0
      (bind _asbp_projectile_trace (Utilities|Casting|CastToBP_ProjectileTrace (Components|GetOwner)))
      (EventDispatchers|BindEventtoProjectilePool _asbp_projectile_trace (delegate Custom|RemoveOrAdd)))
    (:then_1
      (CallFunction|CreateProjectilePool))))