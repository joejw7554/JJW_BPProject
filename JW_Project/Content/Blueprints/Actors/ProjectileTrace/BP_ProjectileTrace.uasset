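; BP_ProjectileTrace is a bullet projectile actor that flies at a configurable speed and expires after a set lifetime.
; The construction script and BeginPlay both copy InitSpeed into the ProjectileMovement initial and max speeds, and BeginPlay also applies LifeTime as the lifespan.
; Overlaps on the BulletProjectile component destroy the actor unless the other actor is tagged Player, with no damage applied.
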(event OnComponentBeginOverlap(BulletProjectile)
  (params (OverlappedComponent :type Primitive%20Component%20Object%20Reference) (OtherActor :type Actor%20Object%20Reference) (OtherComp :type Primitive%20Component%20Object%20Reference) (OtherBodyIndex :type Integer) (bFromSweep :type Boolean) (SweepResult :type Hit%20Result%20Structure%20%28by%20ref%29))
  (if (not (Actor|ActorHasTag OtherActor "Player"))
    (Actor|DestroyActor)))

(event EventBeginPlay
  (bind _projectilemovement (Variables|Default|GetProjectileMovement))
  (bind _initspeed (Variables|Default|GetInitSpeed))
  (Variables|/Script/Engine.ProjectileMovementComponent|SetInitialSpeed _projectilemovement _initspeed)
  (Variables|/Script/Engine.ProjectileMovementComponent|SetMaxSpeed _projectilemovement _initspeed)
  (Actor|SetLifeSpan (Variables|Default|GetLifeTime)))

(fn ConstructionScript
  (bind _projectilemovement (Variables|Default|GetProjectileMovement))
  (bind _initspeed (Variables|Default|GetInitSpeed))
  (Variables|/Script/Engine.ProjectileMovementComponent|SetInitialSpeed _projectilemovement _initspeed)
  (Variables|/Script/Engine.ProjectileMovementComponent|SetMaxSpeed _projectilemovement _initspeed))