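; BP_WeaponBase is a base weapon Blueprint that handles firing and equip/unequip montages.
; Fire combines a hitscan trace that damages Enemy-tagged actors, a pooled projectile spawn and an attached muzzle flash; the sound event is still an empty stub.
; Both trace and projectile originate from an arrow component fetched from the player pawn at BeginPlay, rather than from the gun's muzzle socket.
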(event Custom|Fire
  (CallFunction|LineTrace)
  (CallFunction|SpawnProjectile)
  (CallFunction|PlayVFX)
  ;[0.15 0.15 0.15 0.5] NotDoneYet
  (CallFunction|PlaySFX))

(event Custom|LineTrace
  (bind _raycaststartcomponent (Variables|Default|GetRayCastStartComponent))
  (bind _returnvalue (Transformation|GetWorldLocation _raycaststartcomponent))
  (bind _outhit (Collision|LineTraceByChannel _returnvalue (+ _returnvalue (* (Math|Vector|GetForwardVector (Transformation|GetWorldRotation _raycaststartcomponent)) (Variables|WeaponProperty|GetWeaponRange))) "TraceTypeQuery1" false 0 "ForDuration"))
  (Utilities|IsValid (.hitactor _outhit)
    (:Is%20Valid
      (if (Actor|ActorHasTag (.hitactor _outhit) "Enemy")
        (Game|Damage|ApplyDamage (.hitactor _outhit) (Variables|WeaponProperty|GetWeaponDamage) 0 self "/Script/Engine.DamageType")))))

(event Custom|PlayVFX
  (Effects|SpawnEmitterAttached "/Game/Assets/MilitaryWeapSilver/FX/P_AssaultRifle_MuzzleFlash.P_AssaultRifle_MuzzleFlash" (Variables|Default|GetGunMesh) "MuzzleSocket" "0, 0, 0" "0, 0, 0" "1.000000,1.000000,1.000000" "SnapToTarget"))

(event Custom|PlaySFX)

(event Custom|PlayEquipMontage
  ;[0.15 0.15 0.15 0.5] Equip Unequip 애니메이션 넣고 몽타주 구현해야함
  (Animation|Montage|PlayMontage 0 (Variables|Montage|GetEquipMontage) (Variables|Montage|GetEquipMontagePlayRate)))

(event Custom|PlayUnequipMontage
  ;[0.15 0.15 0.15 0.5] Equip Unequip 애니메이션 넣고 몽타주 구현해야함
  (Animation|Montage|PlayMontage 0 (Variables|Montage|GetUnequipMontage) (Variables|Montage|GetEquipMontagePlayRate)))

(event Custom|SpawnProjectile
  (Default|GetObject (Variables|Default|GetBP_ProjectilePoolComponent) (Transformation|GetWorldTransform (Variables|Default|GetRayCastStartComponent))))

(event EventBeginPlay
  (bind _arrowcomp (Class|BPIPlayer|GetArrowComponent(Message) (Game|Player|GetPlayerPawn 0)))
  (Variables|Default|SetRayCastStartComponent _arrowcomp))

(fn ConstructionScript)