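; BP_AKS is a child weapon Blueprint for the AKS, configured to use assault rifle attachment sockets.
; Its construction script runs the parent's, then sets the weapon and holster socket names and the equip montage play rate.
; The event graph adds no logic of its own: BeginPlay only calls the parent, and the overlap and Tick events are disabled.
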(event EventBeginPlay
  (|CallParentFunction))

(event Collision|EventActorBeginOverlap
  (params (OtherActor :type Actor%20Object%20Reference))
  (|CallParentFunction OtherActor) ; This node is disabled and will not be called.\nDrag off pins to build functionality.
)

(event EventTick
  (params (DeltaSeconds :type Float%20%28single-precision%29))
  (|CallParentFunction DeltaSeconds) ; This node is disabled and will not be called.\nDrag off pins to build functionality.
)

(fn ConstructionScript
  (Utilities|FlowControl|Sequence
    (:then_0
      (|CallParentFunction))
    (:then_1
      (Variables|Default|SetWeaponSocketName "ARWeaponSocket")
      (Variables|Default|SetHolsterSocketName "ARHolsterSocket")
      (Variables|Default|SetEquipMontagePlayRate 1.0))))