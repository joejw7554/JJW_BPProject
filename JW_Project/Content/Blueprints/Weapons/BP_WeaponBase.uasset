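; Base weapon actor that handles firing, ammo, equip and reload montages, and attachment between the owning character's hand and holster sockets.
; Fire is blocked during actions or without ammo; otherwise it line-traces to damage "Enemy"-tagged actors, pulls a pooled projectile, plays effects and decrements ammo.
; Trace and projectile originate from an arrow component fetched from player pawn 0.
; Ammo changes are broadcast to UI, and a left-hand IK location is exposed.
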(event Custom|Fire
  (bind _tickticksfx (Variables|Default|GetTickTickSFX))
  (if (CallFunction|IsDoingAction)
    (Audio|SpawnSoundatLocation "/Game/Audio/Sounds/Weapons/Rifle/MS_TickTickSound.MS_TickTickSound" (Transformation|GetActorLocation) "0, 0, 0" 1.0 1.0 0.0 0 0)
    (elif (CallFunction|HasAmmo)
      (CallFunction|LineTrace)
      (CallFunction|SpawnProjectile)
      (CallFunction|PlayVFX)
      (CallFunction|PlaySFX)
      (Variables|WeaponProperty|SetCurrentAmmo (Math|Integer|Clamp(Integer) (- (Variables|WeaponProperty|GetCurrentAmmo) 1) 0 30))
      (CallFunction|UpdateWeaponUI)
      (else
        (Utilities|IsValid _tickticksfx
          (:Is%20Valid
            (Audio|SpawnSoundatLocation _tickticksfx (Transformation|GetActorLocation) "0, 0, 0" 1.0 1.0 0.0 0 0)))))))

(event Custom|LineTrace
  (bind _raycaststartcomponent (Variables|Default|GetRayCastStartComponent))
  (bind _returnvalue (Transformation|GetWorldLocation _raycaststartcomponent))
  (bind _outhit (Collision|LineTraceByChannel _returnvalue (+ _returnvalue (* (Math|Vector|GetForwardVector (Transformation|GetWorldRotation _raycaststartcomponent)) (Variables|WeaponProperty|GetWeaponRange))) "TraceTypeQuery1" false 0 "ForDuration"))
  (Utilities|IsValid (.hitactor _outhit)
    (:Is%20Valid
      (if (Actor|ActorHasTag (.hitactor _outhit) "Enemy")
        (Game|Damage|ApplyDamage (.hitactor _outhit) (Variables|WeaponProperty|GetWeaponDamage) 0 self "/Script/Engine.DamageType")))))

(event Custom|PlayVFX
  (Effects|SpawnEmitterAttached "/Game/Assets/MilitaryWeapSilver/FX/P_AssaultRifle_MuzzleFlash.P_AssaultRifle_MuzzleFlash" (Variables|Default|GetGunMesh) (Variables|WeaponProperty|GetMuzzleSocketName) "0, 0, 0" "0, 0, 0" "1.000000,1.000000,1.000000" "SnapToTarget"))

(event Custom|PlaySFX
  (Audio|SpawnSoundatLocation (Variables|Default|GetGunSound) (Transformation|GetActorLocation) "0, 0, 0" 1.0 1.0 0.0 0 0))

(event Custom|UpdateWeaponUI
  (Default|CallOnUpdateWeaponUI (Variables|Default|GetWeaponTypeName) (Variables|WeaponProperty|GetCurrentAmmo)))

(event Custom|PlayEquipMontage
  (bind _equipmontage (Variables|Montage|GetEquipMontage))
  ;[0.15 0.15 0.15 0.5] 애니메이션
  (Utilities|IsValid _equipmontage
    (:Is%20Valid
      (Animation|Montage|PlayMontage (Variables|Default|GetOwnerMesh) _equipmontage (Variables|Montage|GetEquipMontagePlayRate)
        (:then
          (CallFunction|UpdateWeaponUI))))))

(event Custom|SpawnProjectile
  ;[0.15 0.15 0.15 0.5] Comment
  (Default|GetObject (Variables|Default|GetBP_ProjectilePoolComponent) (Transformation|GetWorldTransform (Variables|Default|GetRayCastStartComponent))))

(event Custom|PlayReloadMontage
  (bind _reloadmontage (Variables|Montage|GetReloadMontage))
  ;[0.15 0.15 0.15 0.5] 애니메이션
  (if (!= (Variables|WeaponProperty|GetCurrentAmmo) (Variables|WeaponProperty|GetMaxAmmo))
    (Utilities|IsValid _reloadmontage
      (:Is%20Valid
        (Animation|Montage|PlayMontage (Variables|Default|GetOwnerMesh) _reloadmontage (Variables|Montage|GetReloadMontagePlayRate)
          (:then
            (CallFunction|UpdateWeaponUI)))))))

(event EventBeginPlay
  (bind _arrowcomp (Class|BPIPlayer|GetArrowComponent(Message) (Game|Player|GetPlayerPawn 0)))
  (Variables|Default|SetRayCastStartComponent _arrowcomp)
  (bind _ascharacter (Utilities|Casting|CastToCharacter (Components|GetOwner))
    (:then
      (bind _output_get (Variables|Default|SetOwnerMesh (Variables|/Script/Engine.Character|GetMesh _ascharacter)))
      (Transformation|AttachComponentToComponent _output_get (Variables|WeaponProperty|GetHolsterSocketName) "SnapToTarget" "SnapToTarget" "SnapToTarget" true)
      (Variables|WeaponProperty|SetCurrentAmmo (Variables|WeaponProperty|GetMaxAmmo)))
    (:CastFailed
      (Development|PrintString "WEaponBase CastFailed"))))

(fn ConstructionScript)

(fn AttachWeapontoMesh
  (params (OwnerMesh :type Skeletal%20Mesh%20Component%20Object%20Reference) (SocketToAttach :type Name))
  (Transformation|AttachComponentToComponent OwnerMesh SocketToAttach "SnapToTarget" "SnapToTarget" "SnapToTarget" true))

(fn IsDoingAction
  (if (Variables|Action|GetInAction)
    (return true)
    (else
      (return false))))

(fn BeginEquip
  (bind _weaponsocketname (Variables|WeaponProperty|GetWeaponSocketName))
  (if (!= _weaponsocketname "Name_None")
    (CallFunction|AttachWeapontoMesh (Variables|Default|GetOwnerMesh) _weaponsocketname)))

(fn EndAction
  (Variables|Action|SetInAction false))

(fn BeginUnequip
  (bind _holstersocketname (Variables|WeaponProperty|GetHolsterSocketName))
  (if (!= _holstersocketname "Name_None")
    (CallFunction|AttachWeapontoMesh (Variables|Default|GetOwnerMesh) _holstersocketname)))

(fn GetLeftHandLocation
  (return (Variables|WeaponProperty|GetIKLeftHandLocation)))

(fn HasAmmo
  (return (> (Variables|WeaponProperty|GetCurrentAmmo) 0)))

(fn SetAmmo
  (Variables|WeaponProperty|SetCurrentAmmo (Variables|WeaponProperty|GetMaxAmmo))
  (CallFunction|UpdateWeaponUI))