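; BP_BaseEnemy is a base enemy Blueprint that tracks health and reacts to incoming damage.
; CurrentHP starts at MaxHP, and AnyDamage subtracts damage, clamped between zero and the current value so a hit cannot raise health.
; CheckDead then branches on zero health, with debug prints standing in for the death and hit animations.
; Nothing destroys or disables the enemy at zero health, and the overlap event is empty.
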(event Custom|CheckDead
  (if (<= (Variables|Default|GetCurrentHP) 0.0)
    ;[0.15 0.15 0.15 0.5] PlayDeadAnim
    (Development|PrintString "I'm Dead Stop Shooting")
    (else
      ;[0.15 0.15 0.15 0.5] PlayHitAnim
      (Development|PrintString "Not Dead"))))

(event EventBeginPlay
  (Variables|Default|SetCurrentHP (Variables|Default|GetMaxHP)))

(event Collision|EventActorBeginOverlap
  (params (OtherActor :type Actor%20Object%20Reference)))

(event Game|Damage|EventAnyDamage
  (params (Damage :type Float%20%28single-precision%29) (DamageType :type Damage%20Type%20Object%20Reference) (InstigatedBy :type Controller%20Object%20Reference) (DamageCauser :type Actor%20Object%20Reference))
  (Variables|Default|SetCurrentHP (Math|Float|Clamp(Float) (- (Variables|Default|GetCurrentHP) Damage) 0.0 (Variables|Default|GetCurrentHP)))
  (CallFunction|CheckDead))

(fn ConstructionScript)