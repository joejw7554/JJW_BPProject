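; Base enemy Blueprint that tracks hit points and responds to damage.
; CurrentHP starts at MaxHP on BeginPlay, and AnyDamage subtracts damage, clamped between zero and the current value so it cannot rise.
; Each hit then calls IsDead, which checks for zero HP but has no death logic yet.
; The overlap event and construction script are empty.
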(event Custom|Is%20Dead
  (if (<= (Variables|Default|GetCurrentHP) 0.0)
    _))

(event EventBeginPlay
  (Variables|Default|SetCurrentHP (Variables|Default|GetMaxHP)))

(event Collision|EventActorBeginOverlap
  (params (OtherActor :type Actor%20Object%20Reference)))

(event Game|Damage|EventAnyDamage
  (params (Damage :type Float%20%28single-precision%29) (DamageType :type Damage%20Type%20Object%20Reference) (InstigatedBy :type Controller%20Object%20Reference) (DamageCauser :type Actor%20Object%20Reference))
  (Variables|Default|SetCurrentHP (Math|Float|Clamp(Float) (- (Variables|Default|GetCurrentHP) Damage) 0.0 (Variables|Default|GetCurrentHP)))
  (CallFunction|IsDead))

(fn ConstructionScript)